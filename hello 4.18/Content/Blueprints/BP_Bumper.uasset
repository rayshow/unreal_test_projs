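; Pinball-style bumper actor that knocks a BP_Ball away when the ball overlaps it.
; Bump applies a velocity-change impulse along the direction from the bumper to the ball and plays an attached hit sound.
; A timeline then drives the mechanism's downward movement, a point light's intensity and an emissive boost on the top's dynamic material, which is created in the construction script.
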(event `self.ReceiveActorBeginOverlap`
  (params (OtherActor :type "Actor Object Reference"))
  (bind _asbp_ball (cast `/Game/Blueprints/BP_Ball` OtherActor))
  (`self.Bump` _asbp_ball))

(event `Bump`
  (params (Ball :type "/Game/Blueprints/BP_Ball Object Reference"))
  (`PrimitiveComponent.AddImpulse` (`/Game/Blueprints/BP_Ball.Ball` Ball) (* (`KismetMathLibrary.GetDirectionUnitVector` (`self.K2_GetActorLocation`) (`self.K2_GetActorLocation` Ball)) 3000.0) "None" true)
  (`GameplayStatics.SpawnSoundAttached` "/Game/Assets/Sounds/BumpHit.BumpHit" (`self.BumperBase`))
  (bind (_direction _bumpalpha) (`Timeline|BumpAlpha` :!via `PlayFromStart`)
    (:`Update`
      (`SceneComponent.K2_SetRelativeLocation` (`self.BumperMachanism`) (`KismetMathLibrary.VLerp` (0.0 0.0 0.0) (0.0 0.0 -70.0) _bumpalpha) false false)
      (`LightComponent.SetIntensity` (`self.PointLight`) (`KismetMathLibrary.Lerp` 0.0 10000.0 _bumpalpha))
      (`MaterialInstanceDynamic.SetScalarParameterValue` (`self.BumpTopMid`) "EmissiveBoost" (`KismetMathLibrary.Lerp` 0.0 20.0 _bumpalpha)))))

(fn `UserConstructionScript`
  (bind _returnvalue (`PrimitiveComponent.CreateDynamicMaterialInstance` (`self.BumperBase`) 1 "/Game/Assets/M_BumperTop.M_BumperTop"))
  (set `self.BumpTopMid` _returnvalue))